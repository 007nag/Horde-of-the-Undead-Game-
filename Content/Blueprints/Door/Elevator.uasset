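; Elevator actor with two sliding doors that closes when the player enters its Box, then travels to the MoveTo actor's location.
; Timelines nudge both doors along world X by a fixed step per update, with a Bool blocking retriggers while closing.
; When closing finishes, a third timeline lerps the actor from its current location toward MoveTo.
; OpenDoor is a separate event, not called automatically on arrival.
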(event OnComponentBeginOverlap(Box)
  (params (OverlappedComponent :type Primitive%20Component%20Object%20Reference) (OtherActor :type Actor%20Object%20Reference) (OtherComp :type Primitive%20Component%20Object%20Reference) (OtherBodyIndex :type Integer) (bFromSweep :type Boolean) (SweepResult :type Hit%20Result%20Structure%20%28by%20ref%29))
  (bind _door1 (Variables|Default|Getdoor1))
  (bind _door2 (Variables|Default|Getdoor2))
  (bind _returnvalue (Transformation|GetWorldLocation _door2))
  (bind _returnvalue_2 (Transformation|GetWorldLocation _door1))
  (if (and (not (Variables|Default|Getbool)) (== OtherActor (Game|GetPlayerCharacter 0)))
    (Variables|Default|Setbool true)
    (Timeline|Timeline_1 PlayFromStart
      (:Update
        (Transformation|SetWorldLocation _door1 (Math|Vector|MakeVector (+ (.x _returnvalue_2) 1.0) (.y _returnvalue_2) (.z _returnvalue_2)) false false)
        (Transformation|SetWorldLocation _door2 (Math|Vector|MakeVector (+ (.x _returnvalue) -1.0) (.y _returnvalue) (.z _returnvalue)) false false))
      (:Finished
        (Variables|Default|Setbool false)
        (Utilities|FlowControl|Sequence
          (:then_0
            (bind _newtrack_0 (Timeline|Timeline_2 SetNewTime)
              (:Update
                (Transformation|SetActorLocation (Math|Vector|Lerp(Vector) (Transformation|GetActorLocation) (Transformation|GetActorLocation (Variables|Default|Getmove_to)) _newtrack_0) false false))))
          (:then_1
            (Timeline|Timeline_2 PlayFromStart)))))))

(event EventBeginPlay)

(event Collision|EventActorBeginOverlap
  (params (OtherActor :type Actor%20Object%20Reference)))

(event EventTick
  (params (DeltaSeconds :type Float%20%28single-precision%29)))

(event EventOpenDoor
  (bind _door1 (Variables|Default|Getdoor1))
  (bind _door2 (Variables|Default|Getdoor2))
  (bind _returnvalue (Transformation|GetWorldLocation _door1))
  (bind _returnvalue_2 (Transformation|GetWorldLocation _door2))
  (Timeline|Timeline_0 PlayFromStart
    (:Update
      (Transformation|SetWorldLocation _door1 (Math|Vector|MakeVector (+ (.x _returnvalue) -1.0) (.y _returnvalue) (.z _returnvalue)) false false)
      (Transformation|SetWorldLocation _door2 (Math|Vector|MakeVector (+ (.x _returnvalue_2) 1.0) (.y _returnvalue_2) (.z _returnvalue_2)) false false))))

(event EventCloseDoor
  (bind _door1 (Variables|Default|Getdoor1))
  (bind _door2 (Variables|Default|Getdoor2))
  (bind _returnvalue (Transformation|GetWorldLocation _door2))
  (bind _returnvalue_2 (Transformation|GetWorldLocation _door1))
  (if (and (not (Variables|Default|Getbool)) (== (stale OnComponentBeginOverlap(Box) OtherActor) (Game|GetPlayerCharacter 0)))
    (Variables|Default|Setbool true)
    (Timeline|Timeline_1 PlayFromStart
      (:Update
        (Transformation|SetWorldLocation _door1 (Math|Vector|MakeVector (+ (.x _returnvalue_2) 1.0) (.y _returnvalue_2) (.z _returnvalue_2)) false false)
        (Transformation|SetWorldLocation _door2 (Math|Vector|MakeVector (+ (.x _returnvalue) -1.0) (.y _returnvalue) (.z _returnvalue)) false false))
      (:Finished
        (Variables|Default|Setbool false)
        (Utilities|FlowControl|Sequence
          (:then_0
            (bind _newtrack_0 (Timeline|Timeline_2 SetNewTime)
              (:Update
                (Transformation|SetActorLocation (Math|Vector|Lerp(Vector) (Transformation|GetActorLocation) (Transformation|GetActorLocation (Variables|Default|Getmove_to)) _newtrack_0) false false))))
          (:then_1
            (Timeline|Timeline_2 PlayFromStart)))))))

(fn ConstructionScript)