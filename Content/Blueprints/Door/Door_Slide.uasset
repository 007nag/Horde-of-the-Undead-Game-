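; Sliding door Blueprint that moves along its right vector on OpenDoor and returns to its starting position on CloseDoor.
; Opening adds a fixed step on each timeline update, so travel depends on update count, and records the end location when finished.
; Closing uses a second timeline's track to lerp from that recorded location back to the one saved at BeginPlay.
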(event EventBeginPlay
  (Variables|Default|Setinitial_Loc (Transformation|GetWorldLocation (Variables|Default|GetDefaultSceneRoot))))

(event EventOpenDoor
  (bind _defaultsceneroot (Variables|Default|GetDefaultSceneRoot))
  (bind _returnvalue (Transformation|GetWorldLocation _defaultsceneroot))
  (Timeline|Timeline_0 PlayFromStart
    (:Update
      (Transformation|SetWorldLocation _defaultsceneroot (+ (* (Math|Vector|Normalize (Math|Vector|GetRightVector _defaultsceneroot)) 5) _returnvalue) false false))
    (:Finished
      (Variables|Default|Setlast_loc _returnvalue))))

(event EventCloseDoor
  (bind _newtrack_0 (Timeline|Timeline_1 PlayFromStart)
    (:Update
      (Transformation|SetWorldLocation (Variables|Default|GetDefaultSceneRoot) (Math|Vector|Lerp(Vector) (Variables|Default|Getlast_loc) (Variables|Default|Getinitial_Loc) _newtrack_0) false false))))

(fn ConstructionScript
  (|CallParentFunction))