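; Builder tool that stacks static meshes in a grid of rows and columns projected onto the surface below.
; When Generate is set, the construction script derives spacing from fixed offset or total length, optionally centered, then line-traces down from each point.
; Hits get mesh components aligned to the impact normal, with incremental and seeded random transforms and cycled or random meshes.
; PlacePermanentCopies spawns those components as separate StaticMeshActors.
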(event EventBeginPlay)

(event Collision|EventActorBeginOverlap
  (params (OtherActor :type Actor%20Object%20Reference)))

(event EventTick
  (params (DeltaSeconds :type Float%20%28single-precision%29)))

(fn ConstructionScript
  (bind _locationbase (Variables|Extra|GetLocationBase))
  (bind _length (Variables|Mode:Length|GetLength))
  (bind _seed (Variables|Base|GetSeed))
  (bind _locationoffset (Variables|Mode:Offset|GetLocationOffset))
  (bind (_x _y) (Math|Vector|BreakVector _locationoffset))
  (bind (_x_2 _y_2) (Math|Vector|BreakVector _length))
  (if (Variables|Base|GetGenerate)
    (Utilities|FlowControl|Sequence
      (:then_0
        (LocalVariables|SetOffset (Utilities|Select :Index (Variables|Base|GetMode) :NewEnumerator0 (Variables|Mode:Offset|GetLocationOffset) :NewEnumerator1 (Math|Vector|MakeVector (/ _x_2 (Math|Float|Max(Float) (Math|Conversions|ToFloat(Integer) (- (Variables|Base|GetRows) 1)) 1.0)) (/ _y_2 (Math|Float|Max(Float) (Math|Conversions|ToFloat(Integer) (- (Variables|Base|GetColumns) 1)) 1.0)) 0.0)))
        (LocalVariables|SetBase (Math|Vector|SelectVector (+ (Utilities|Select :Index (Variables|Base|GetMode) :NewEnumerator0 (/ (Math|Vector|MakeVector (* _x (Math|Conversions|ToFloat(Integer) (- (Variables|Base|GetRows) 1))) (* _y (Math|Conversions|ToFloat(Integer) (- (Variables|Base|GetColumns) 1))) 0.0) -2.0) :NewEnumerator1 (/ (Variables|Mode:Length|GetLength) -2.0)) _locationbase) _locationbase (Variables|Base|GetCenter))))
      (:then_1
        (for _index (range 0 (- (Variables|Base|GetRows) 1))
          (for _index_2 (range 0 (- (Variables|Base|GetColumns) 1))
            (bind (_outhit _returnvalue) (Collision|LineTraceForObjects (CallFunction|RelativeLoctoWorld (+ (Math|Vector|MakeVector (* _index (.X (Math|Vector|BreakVector (LocalVariables|GetOffset)))) (* _index_2 (.Y (Math|Vector|BreakVector (LocalVariables|GetOffset)))) 0.0) (LocalVariables|GetBase)) (Transformation|GetActorTransform)) (- (CallFunction|RelativeLoctoWorld (+ (Math|Vector|MakeVector (* _index (.X (Math|Vector|BreakVector (LocalVariables|GetOffset)))) (* _index_2 (.Y (Math|Vector|BreakVector (LocalVariables|GetOffset)))) 0.0) (LocalVariables|GetBase)) (Transformation|GetActorTransform)) "0,0.000000,16384.000000") (Variables|Base|GetTraceTypes) false 0 "None"))
            (if _returnvalue
              (bind _returnvalue_2 (AddComponent|AddStaticMeshComponent true (CallFunction|CombineTransform (Math|Transform|MakeTransform (.ImpactPoint (Collision|BreakHitResult _outhit)) (Math|Rotator|SelectRotator (Math|Rotator|CombineRotators (Math|Rotator|CombineRotators (* (Variables|Extra|GetRotationOffset) (+ _index_2 (* _index (Variables|Base|GetColumns)))) (Variables|Extra|GetRotationBase)) (Math|Rotator|MakeRotfromZ (.ImpactNormal (Collision|BreakHitResult _outhit)))) (Math|Rotator|MakeRotfromZ (.ImpactNormal (Collision|BreakHitResult _outhit))) (Variables|Default|GetFollowRotation)) (+ (* (Variables|Extra|GetScaleOffset) (+ _index_2 (* _index (Variables|Base|GetColumns)))) (Variables|Extra|GetScaleBase))) (Math|Transform|MakeTransform (CallFunction|RandomVectorSeeded (Variables|Random|GetMinRandomLocation) (Variables|Random|GetMaxRandomLocation) _seed) (CallFunction|RandomRotSeeded (Variables|Random|GetMinRandomRotation) (Variables|Random|GetMaxRandomRotation) _seed) (CallFunction|RandomVectorSeeded (Variables|Random|GetMinRandomScale) (Variables|Random|GetMaxRandomScale) _seed)))))
              (switch Utilities|FlowControl|Switch|SwitchonESelect (Variables|Base|GetMeshSelection)
                (:NewEnumerator0
                  (Components|StaticMesh|SetStaticMesh _returnvalue_2 (Utilities|Array|Get(acopy) (Variables|Base|GetMesh) (LocalVariables|GetpIndex)))
                  (LocalVariables|SetpIndex (Math|Integer|%(Integer) (+ (LocalVariables|GetpIndex) 1) (Utilities|Array|Length (Variables|Base|GetMesh)))))
                (:NewEnumerator1
                  (Components|StaticMesh|SetStaticMesh _returnvalue_2 (Utilities|RandomItemSeeded (Variables|Base|GetMesh) (Variables|Base|GetSeed)))))
              (Utilities|Array|Add (Variables|Default|GetMeshComps) _returnvalue_2))))))))

(fn PlacePermanentCopies
  (for _array_element (Variables|Default|GetMeshComps)
    (bind _returnvalue (Game|SpawnActorfromClass "/Script/Engine.StaticMeshActor" (Transformation|GetWorldTransform _array_element) "AlwaysSpawn" 0 0))
    (Components|StaticMesh|SetStaticMesh (Variables|/Script/Engine.StaticMeshActor|GetStaticMeshComponent _returnvalue) (Variables|/Script/Engine.StaticMeshComponent|GetStaticMesh _array_element))))