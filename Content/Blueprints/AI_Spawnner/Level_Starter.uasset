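; Level_Starter is a trigger actor that runs one combat phase of a level when the player enters its box.
; The first overlap saves a checkpoint, restores the player and closes its door (skipped for the start phase), then spawns a boss or configures an AI_Spawnner.
; On phase completion, it opens the next starter's door, or in the final phase saves progress and loads the next level after a delay.
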(event OnComponentBeginOverlap(Box)
  (params (OverlappedComponent :type Primitive%20Component%20Object%20Reference) (OtherActor :type Actor%20Object%20Reference) (OtherComp :type Primitive%20Component%20Object%20Reference) (OtherBodyIndex :type Integer) (bFromSweep :type Boolean) (SweepResult :type Hit%20Result%20Structure%20%28by%20ref%29))
  (if (and (== OtherActor (Game|GetPlayerCharacter 0)) (not (Variables|Default|Getbool_1)))
    (Variables|Default|Setbool_1 true)
    (if (!= (Variables|Default|Getstart/middle/end) 0)
      (bind _returnvalue (SaveGame|CreateSaveGameObject "/Game/Blueprints/SaveGame/SaveGame_Obj.SaveGame_Obj_C"))
      (bind _returnvalue_2 (Game|GetCurrentLevelName true))
      (Variables|/Game/Blueprints/SaveGame/SaveGame_Obj.SaveGame_Obj_C|SetLevel_Name _returnvalue (Utilities|String|StringToName _returnvalue_2))
      (CallFunction|Restore)
      (Variables|/Game/Blueprints/SaveGame/SaveGame_Obj.SaveGame_Obj_C|SetLevelStart/Not _returnvalue false)
      (Variables|/Game/Blueprints/SaveGame/SaveGame_Obj.SaveGame_Obj_C|SetLocation _returnvalue (Transformation|GetWorldLocation (Variables|Default|GetSphere1)))
      (SaveGame|SaveGametoSlot _returnvalue "SaveGame")
      (if (Variables|/Game/Blueprints/Door/Door_Base.Door_Base_C|Getcan_close (Variables|Default|Getdoor_to_open))
        (CallFunction|CloseDoor)))
    (if (Variables|Default|Getboss)
      (CallFunction|SpawnBoss)
      (else
        (bind _returnvalue_3 (Game|SpawnActorfromClass "/Game/Blueprints/AI_Spawnner/AI_Spawnner.AI_Spawnner_C" (Transformation|GetActorTransform) "Undefined" 0 0))
        (bind _output_get (Variables|Default|SetAI_spawnner _returnvalue_3))
        (Variables|/Game/Blueprints/AI_Spawnner/AI_Spawnner.AI_Spawnner_C|Setlocation_array _output_get (Variables|Default|Getlocation_array))
        (Variables|/Game/Blueprints/AI_Spawnner/AI_Spawnner.AI_Spawnner_C|SetLevel%20Starter _output_get self)
        (Variables|/Game/Blueprints/AI_Spawnner/AI_Spawnner.AI_Spawnner_C|SetAlly/Zombie _output_get (Variables|Default|GetAlly/Zombie))
        (Default|BeginEvent _output_get)))))

(event Custom|Phase_complete
  (bind _next_level_name (Variables|Default|Getnext_level_name))
  ;[1 1 1] PHase COmplete
  (Utilities|FlowControl|DoOnce false
    (:Completed
      (if (== (Variables|Default|Getstart/middle/end) 2)
        (bind _returnvalue (SaveGame|CreateSaveGameObject "/Game/Blueprints/SaveGame/SaveGame_Obj.SaveGame_Obj_C"))
        (Variables|/Game/Blueprints/SaveGame/SaveGame_Obj.SaveGame_Obj_C|SetLevel_Name _returnvalue _next_level_name)
        (Variables|/Game/Blueprints/SaveGame/SaveGame_Obj.SaveGame_Obj_C|SetLevelStart/Not _returnvalue true)
        (SaveGame|SaveGametoSlot _returnvalue "SaveGame")
        (Utilities|FlowControl|Delay 5.0)
        (Game|OpenLevel(byName) _next_level_name)
        (else
          (CallFunction|OpenDoor (Variables|Default|Getnext_level_starter)))))))

(event Custom|open_door
  (bind _door_to_open (Variables|Default|Getdoor_to_open))
  (Variables|/Game/Blueprints/Door/Door_Base.Door_Base_C|Setcan_close _door_to_open true)
  (Default|OpenDoor _door_to_open))

(event Custom|close_door
  (Default|CloseDoor (Variables|Default|Getdoor_to_open)))

(event Custom|spawn_boss
  (bind _self self)
  (bind _location_array (Variables|Default|Getlocation_array))
  (bind _loc_array (Variables|/Game/Blueprints/AI_Spawnner/Location_Array.Location_Array_C|GetLoc_Array _location_array))
  (bind _output (Utilities|Array|Get(acopy) _loc_array))
  (bind _returnvalue (Transformation|GetActorLocation _output))
  ;[1 1 1] Spawn Boss
  (switch int (Variables|Default|Getdoc/saber/zombie)
    (:0
      (bind _returnvalue_2 (Game|SpawnActorfromClass "/Game/Blueprints/Characters/Enemy/Enemy_3/Enemy_3.Enemy_3_C" (Math|Transform|MakeTransform _returnvalue "0, 0, 0" "1,1,1") "Undefined" 0 0))
      (Variables|/Game/Blueprints/Characters/Enemy/Enemy_3/Enemy_3.Enemy_3_C|Setlevel_starter _returnvalue_2 _self))
    (:1
      (bind _returnvalue_3 (Game|SpawnActorfromClass "/Game/Blueprints/Characters/Enemy/Enemy_2/Enemy_2.Enemy_2_C" (Math|Transform|MakeTransform _returnvalue "0, 0, 0" "1,1,1") "Undefined" 0 0))
      (Variables|/Game/Blueprints/Characters/Enemy/Enemy_2/Enemy_2.Enemy_2_C|Setlevel_starter _returnvalue_3 _self))))

(event Custom|restore
  (bind _returnvalue (Game|GetPlayerCharacter 0))
  (if (Variables|Default|Getplayer/doctor)
    (bind _asfirst_person_character (Utilities|Casting|CastToFirstPersonCharacter _returnvalue))
    (Default|Restore _asfirst_person_character)
    (else
      (bind _asenemy_3_playable (Utilities|Casting|CastToEnemy_3_Playable _returnvalue))
      (Default|Restore _asenemy_3_playable))))

(event EventBeginPlay)

(event Collision|EventActorBeginOverlap
  (params (OtherActor :type Actor%20Object%20Reference)))

(event EventTick
  (params (DeltaSeconds :type Float%20%28single-precision%29)))

(fn ConstructionScript)