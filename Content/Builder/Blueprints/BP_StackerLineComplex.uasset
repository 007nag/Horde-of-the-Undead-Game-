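; Builder Blueprint that stacks static mesh components in a line when constructed with Generate enabled.
; Two modes space a set Amount by a per-item offset or across a Length along a Direction, with optional centering.
; Each transform combines incremental rotation and scale with seeded random jitter, and meshes are picked cyclically or randomly from an array.
; PlacePermanentCopies spawns the generated meshes as standalone StaticMeshActors.
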(event EventBeginPlay)

(event Collision|EventActorBeginOverlap
  (params (OtherActor :type Actor%20Object%20Reference)))

(event EventTick
  (params (DeltaSeconds :type Float%20%28single-precision%29)))

(fn ConstructionScript
  (bind _mesh (Variables|Base|GetMesh))
  (bind _locationbase (Variables|Extra|GetLocationBase))
  (bind _seed (Variables|Base|GetSeed))
  (bind _seed_2 (Variables|Base|GetSeed))
  (bind _returnvalue (Utilities|Array|Length _mesh))
  (if (Variables|Base|GetGenerate)
    (Utilities|Array|Clear (Variables|Default|GetMeshComps))
    (switch Utilities|FlowControl|Switch|SwitchonESimplePlacement (Variables|Base|GetMode)
      (:NewEnumerator0
        (for _index (range 0 (- (Variables|Base|GetAmount) 1))
          (bind _returnvalue_2 (AddComponent|AddStaticMeshComponent false (CallFunction|CombineTransform (Math|Transform|MakeTransform (CallFunction|RandomVectorSeeded (Variables|Random|GetMinRandomLocation) (Variables|Random|GetMaxRandomLocation) _seed) (CallFunction|RandomRotSeeded (Variables|Random|GetMinRandomRotation) (Variables|Random|GetMaxRandomRotation) _seed) (CallFunction|RandomVectorSeeded (Variables|Random|GetMinRandomScale) (Variables|Random|GetMaxRandomScale) _seed)) (Math|Transform|MakeTransform (+ (Math|Vector|SelectVector (+ (* (Variables|Mode:Offset|GetLocationOffset) (/ (- (Math|Conversions|ToFloat(Integer) (Variables|Base|GetAmount)) 1.0) -2.0)) _locationbase) _locationbase (Variables|Base|GetCenter)) (* (Variables|Mode:Offset|GetLocationOffset) _index)) (Math|Rotator|CombineRotators (* (Variables|Extra|GetRotationOffset) _index) (Variables|Extra|GetRotationBase)) (+ (* (Variables|Extra|GetScaleOffset) _index) (Variables|Extra|GetScaleBase))))))
          (Components|StaticMesh|SetStaticMesh _returnvalue_2 (Utilities|Select :Index (Variables|Base|GetMeshSelection) :NewEnumerator0 (Utilities|Array|Get(acopy) _mesh (Math|Integer|%(Integer) _index _returnvalue)) :NewEnumerator1 (Utilities|Array|Get(acopy) _mesh (Class|KismetMathLibrary|RandomIntegerfromStream _returnvalue (Variables|Base|GetSeed)))))
          (Utilities|Array|Add (Variables|Default|GetMeshComps) _returnvalue_2)))
      (:NewEnumerator1
        (for _index_2 (range 0 (- (Variables|Base|GetAmount) 1))
          (bind _returnvalue_3 (AddComponent|AddStaticMeshComponent false (CallFunction|CombineTransform (Math|Transform|MakeTransform (+ (Math|Vector|SelectVector (+ (Variables|Extra|GetLocationBase) (* (Math|Rotator|GetRotationXVector (Variables|Mode:Length|GetDirection)) (+ (/ (Variables|Mode:Length|GetLength) -2.0) (/ (/ (Variables|Mode:Length|GetLength) (Math|Conversions|ToFloat(Integer) (Variables|Base|GetAmount))) 2.0)))) (Variables|Extra|GetLocationBase) (Variables|Base|GetCenter)) (* (* (Math|Rotator|GetRotationXVector (Variables|Mode:Length|GetDirection)) (/ (Variables|Mode:Length|GetLength) (Math|Conversions|ToFloat(Integer) (Variables|Base|GetAmount)))) _index_2)) (Math|Rotator|CombineRotators (* (Variables|Extra|GetRotationOffset) _index_2) (Variables|Extra|GetRotationBase)) (+ (* (Variables|Extra|GetScaleOffset) _index_2) (Variables|Extra|GetScaleBase))) (Math|Transform|MakeTransform (CallFunction|RandomVectorSeeded (Variables|Random|GetMinRandomLocation) (Variables|Random|GetMaxRandomLocation) _seed_2) (CallFunction|RandomRotSeeded (Variables|Random|GetMinRandomRotation) (Variables|Random|GetMaxRandomRotation) _seed_2) (CallFunction|RandomVectorSeeded (Variables|Random|GetMinRandomScale) (Variables|Random|GetMaxRandomScale) _seed_2)))))
          (Components|StaticMesh|SetStaticMesh _returnvalue_3 (Utilities|Select :Index (Variables|Base|GetMeshSelection) :NewEnumerator0 (Utilities|Array|Get(acopy) _mesh (Math|Integer|%(Integer) _index _returnvalue)) :NewEnumerator1 (Utilities|Array|Get(acopy) _mesh (Class|KismetMathLibrary|RandomIntegerfromStream _returnvalue (Variables|Base|GetSeed)))))
          (Utilities|Array|Add (Variables|Default|GetMeshComps) _returnvalue_3))))))

(fn PlacePermanentCopies
  (for _array_element (Variables|Default|GetMeshComps)
    (bind _returnvalue (Game|SpawnActorfromClass "/Script/Engine.StaticMeshActor" (Transformation|GetWorldTransform _array_element) "AlwaysSpawn" 0 0))
    (Components|StaticMesh|SetStaticMesh (Variables|/Script/Engine.StaticMeshActor|GetStaticMeshComponent _returnvalue) (Variables|/Script/Engine.StaticMeshComponent|GetStaticMesh _array_element))))