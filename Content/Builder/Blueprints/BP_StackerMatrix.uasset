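; BP_StackerMatrix is a construction-script builder that fills a 3D grid of rows, columns and levels with instances of one mesh when Generate is on.
; Mode sets spacing from either a fixed per-step offset or a total length divided across the counts, with optional centering around the base location.
; Each instance's rotation and scale accumulate from base values by its flattened grid index, all on one InstancedStaticMesh component.
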(event EventBeginPlay)

(event Collision|EventActorBeginOverlap
  (params (OtherActor :type Actor%20Object%20Reference)))

(event EventTick
  (params (DeltaSeconds :type Float%20%28single-precision%29)))

(fn ConstructionScript
  (bind _locationbase (Variables|Extra|GetLocationBase))
  (bind _length (Variables|Mode:Length|GetLength))
  (bind _locationoffset (Variables|Mode:Offset|GetLocationOffset))
  (bind (_x _y _z) (Math|Vector|BreakVector _locationoffset))
  (bind (_x_2 _y_2 _z_2) (Math|Vector|BreakVector _length))
  (if (Variables|Base|GetGenerate)
    (Utilities|FlowControl|Sequence
      (:then_0
        (LocalVariables|SetOffset (Utilities|Select :Index (Variables|Base|GetMode) :NewEnumerator0 (Variables|Mode:Offset|GetLocationOffset) :NewEnumerator1 (Math|Vector|MakeVector (/ _x_2 (Math|Float|Max(Float) (Math|Conversions|ToFloat(Integer) (- (Variables|Base|GetRows) 1)) 1.0)) (/ _y_2 (Math|Float|Max(Float) (Math|Conversions|ToFloat(Integer) (- (Variables|Base|GetColumns) 1)) 1.0)) (/ _z_2 (Math|Float|Max(Float) (Math|Conversions|ToFloat(Integer) (- (Variables|Base|GetLevels) 1)) 1.0)))))
        (LocalVariables|SetBase (Math|Vector|SelectVector (+ (Utilities|Select :Index (Variables|Base|GetMode) :NewEnumerator0 (/ (Math|Vector|MakeVector (* _x (Math|Conversions|ToFloat(Integer) (- (Variables|Base|GetRows) 1))) (* _y (Math|Conversions|ToFloat(Integer) (- (Variables|Base|GetColumns) 1))) (* _z (Math|Conversions|ToFloat(Integer) (- (Variables|Base|GetLevels) 1)))) -2.0) :NewEnumerator1 (/ (Variables|Mode:Length|GetLength) -2.0)) _locationbase) _locationbase (Variables|Base|GetCenter))))
      (:then_1
        (Components|StaticMesh|SetStaticMesh (Variables|Default|GetInstancedStaticMesh) (Variables|Base|GetMesh))
        (for _index (range 0 (- (Variables|Base|GetLevels) 1))
          (for _index_2 (range 0 (- (Variables|Base|GetRows) 1))
            (for _index_3 (range 0 (- (Variables|Base|GetColumns) 1))
              (Components|InstancedStaticMesh|AddInstance (Variables|Default|GetInstancedStaticMesh) (Math|Transform|MakeTransform (+ (Math|Vector|MakeVector (* _index_2 (.X (Math|Vector|BreakVector (LocalVariables|GetOffset)))) (* _index_3 (.Y (Math|Vector|BreakVector (LocalVariables|GetOffset)))) (* _index (.Z (Math|Vector|BreakVector (LocalVariables|GetOffset))))) (LocalVariables|GetBase)) (Math|Rotator|CombineRotators (* (Variables|Extra|GetRotationOffset) (+ _index_3 (* _index_2 (Variables|Base|GetColumns)) (* _index (* (Variables|Base|GetColumns) (Variables|Base|GetRows))))) (Variables|Extra|GetRotationBase)) (+ (* (Variables|Extra|GetScaleOffset) (+ _index_3 (* _index_2 (Variables|Base|GetColumns)) (* _index (* (Variables|Base|GetColumns) (Variables|Base|GetRows))))) (Variables|Extra|GetScaleBase)))))))))))