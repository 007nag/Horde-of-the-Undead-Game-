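; Ally scheduler Blueprint that takes turns triggering attacks across an array of actors, in the style of round-robin CPU scheduling.
; After a startup delay, a looping chain from BeginPlay calls AttackEvent on the current actor, waits TimeQuantum, then advances the wrapping index.
; Invalid, dead or possessed actors are skipped after a short delay, so only living, unpossessed allies receive attack turns.
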(event EventBeginPlay
  (bind _actors (Variables|Default|GetActors))
  (Utilities|FlowControl|Delay 4.0)
  (Utilities|IsValid (Utilities|Array|Get(acopy) _actors (Variables|Default|Getcurrent_index)) :!label _label
    (:Is%20Valid
      (if (Variables|/Game/Blueprints/Characters/Ally/Ally/Ally_Base.Ally_Base_C|Getis_dead (Utilities|Array|Get(acopy) _actors (Variables|Default|Getcurrent_index)))
        _
        (elif (Variables|/Game/Blueprints/Characters/Ally/Ally/Ally_Base.Ally_Base_C|Getis_possessed (Utilities|Array|Get(acopy) _actors (Variables|Default|Getcurrent_index)))
          _
          (else
            (Default|AttackEvent (Utilities|Array|Get(acopy) _actors (Variables|Default|Getcurrent_index)))
            (Variables|Default|Setcurrent_index (Math|Integer|%(Integer) (+ (Variables|Default|Getcurrent_index) 1) (Utilities|Array|Length _actors)))
            (Utilities|FlowControl|Delay (Variables|Default|Gettime_quantum))
            (goto _label)))))
    (:Is%20Not%20Valid
      _))
  (Variables|Default|Setcurrent_index (Math|Integer|%(Integer) (+ (Variables|Default|Getcurrent_index) 1) (Utilities|Array|Length _actors)))
  (Utilities|FlowControl|Delay 0.5)
  (goto _label))

(event Collision|EventActorBeginOverlap
  (params (OtherActor :type Actor%20Object%20Reference)))

(event EventTick
  (params (DeltaSeconds :type Float%20%28single-precision%29)))

(fn ConstructionScript)