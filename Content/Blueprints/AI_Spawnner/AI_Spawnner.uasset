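; AI spawner that runs a wave of either Ally_1 actors or Enemy_1 zombies, chosen by the AllyZombie flag, and tracks when the wave is cleared.
; On begin_event it shows a remaining-enemies widget and spawns one randomly skinned character at each LocationArray point.
; Ally waves also create an Ally_Scheduler that receives the spawned actors.
; A death counter reports phase completion to LevelStarter once all are dead, destroying any scheduler first.
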(event Custom|Increment_Death_Count
  (bind _ally_scheduler (Variables|Default|GetAlly_scheduler))
  (bind _result (Math|Integer|IncrementInt (Variables|Default|Getdeath_count))
    (:%20%20
      (Math|Integer|DecrementInt (Variables|Default|Getremaining_enemies)
        (:%20%20
          (if (>= _result (Variables|Default|Getmax_length))
            (if (Variables|Default|GetAlly/Zombie)
              (Utilities|IsValid _ally_scheduler
                (:Is%20Valid
                  (Actor|DestroyActor _ally_scheduler))))
            (Default|PhaseComplete (Variables|Default|GetLevel%20Starter))))))))

(event Custom|begin_event
  (bind _zombie_sk_meshes (Variables|Default|GetZombie_SK_meshes))
  (bind _location_array (Variables|Default|Getlocation_array))
  (bind _ally_sk_meshes (Variables|Default|GetAlly_SK_meshes))
  (bind _loc_array (Variables|/Game/Blueprints/AI_Spawnner/Location_Array.Location_Array_C|GetLoc_Array _location_array))
  (bind _returnvalue (Utilities|Array|Length _loc_array))
  (bind _returnvalue_2 (Game|ConstructObjectfromClass "/Game/Blueprints/UI/Remaining_enemies.Remaining_enemies_C" self))
  (UserInterface|Viewport|AddtoViewport _returnvalue_2 0)
  (Variables|/Game/Blueprints/UI/Remaining_enemies.Remaining_enemies_C|SetAI_spawnnner _returnvalue_2 self)
  (Variables|Default|Setremaining_enemies _returnvalue)
  (Variables|Default|Setmax_length _returnvalue)
  (if (Variables|Default|GetAlly/Zombie)
    (bind _returnvalue_3 (Game|SpawnActorfromClass "/Game/Blueprints/AI_Spawnner/Ally_Scheduler.Ally_Scheduler_C" (Transformation|GetActorTransform) "Undefined" 0 0))
    (Variables|Default|SetAlly_scheduler _returnvalue_3)
    (for _array_element _loc_array
      (bind _returnvalue_4 (Game|SpawnActorfromClass "/Game/Blueprints/Characters/Ally/Ally/Ally_1.Ally_1_C" (Math|Transform|MakeTransform (Transformation|GetActorLocation _array_element) "0, 0, 0" "1,1,1") "Undefined" 0 0))
      (Utilities|Array|Add (Variables|Default|GetAlly_array) _returnvalue_4)
      (Class|SkinnedMeshComponent|SetSkeletalMesh (Variables|/Script/Engine.Character|GetMesh _returnvalue_4) (Utilities|Array|Get(acopy) _ally_sk_meshes (Math|Random|RandomInteger (Utilities|Array|Length _ally_sk_meshes))) true)
      (Variables|/Game/Blueprints/Characters/Ally/Ally/Ally_1.Ally_1_C|SetAI_spawnner _returnvalue_4 self))
    (Variables|/Game/Blueprints/AI_Spawnner/Ally_Scheduler.Ally_Scheduler_C|SetActors (Variables|Default|GetAlly_scheduler) (Variables|Default|GetAlly_array))
    (else
      (for _array_element_2 _loc_array
        (bind _returnvalue_5 (Game|SpawnActorfromClass "/Game/Blueprints/Characters/Enemy/Enemy_1/Enemy_1.Enemy_1_C" (Math|Transform|MakeTransform (Transformation|GetActorLocation _array_element_2) "0, 0, 0" "1,1,1") "Undefined" 0 0))
        (Class|SkinnedMeshComponent|SetSkeletalMesh (Variables|/Script/Engine.Character|GetMesh _returnvalue_5) (Utilities|Array|Get(acopy) _zombie_sk_meshes (Math|Random|RandomInteger (Utilities|Array|Length _zombie_sk_meshes))) true)
        (Variables|/Game/Blueprints/Characters/Enemy/Enemy_1/Enemy_1.Enemy_1_C|Setai_spawnner _returnvalue_5 self)))))

(event EventBeginPlay)

(fn ConstructionScript)