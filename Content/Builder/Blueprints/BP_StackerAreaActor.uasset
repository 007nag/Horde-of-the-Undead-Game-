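; Editor-time scatter actor that fills a circular area with child actors from a class list when Generate is on.
; The construction script places each at a seeded random angle, with radius following a power curve.
; TraceDown projects placements onto surfaces with optional normal alignment; otherwise they get random heights up to Height.
; Seeded transform jitter is applied, and classes are picked in rotation or at random.
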(event EventBeginPlay)

(event Collision|EventActorBeginOverlap
  (params (OtherActor :type Actor%20Object%20Reference)))

(event EventTick
  (params (DeltaSeconds :type Float%20%28single-precision%29)))

(fn ConstructionScript
  (bind _seed (Variables|Base|GetSeed))
  (bind _seed_2 (Variables|Base|GetSeed))
  (bind _seed_3 (Variables|Base|GetSeed))
  (bind _amount (Variables|Base|GetAmount))
  (bind _seed_4 (Variables|Base|GetSeed))
  (bind _returnvalue (Math|Random|RandomFloatinRangefromStream 0.0 3.6e+02 _seed_3))
  (bind _returnvalue_2 (Math|Random|RandomFloatinRangefromStream 0.0 3.6e+02 _seed_2))
  (if (Variables|Base|GetGenerate)
    (if (> (Utilities|Array|Length (Variables|Base|GetClasses)) 0)
      (for _index (range 0 (- _amount 1))
        (if (Variables|Base|GetTraceDown)
          (bind (_outhit _returnvalue_3) (Collision|LineTraceForObjects (+ (Transformation|GetActorLocation) (* (+ (* (Transformation|GetActorForwardVector) (Math|Trig|Cos(Degrees) _returnvalue)) (* (Transformation|GetActorRightVector) (Math|Trig|Sin(Degrees) _returnvalue))) (* (Math|Float|Power (/ (Math|Conversions|ToFloat(Integer) (+ _index 1)) (Math|Conversions|ToFloat(Integer) _amount)) (Variables|Base|GetRatio)) (Variables|Base|GetRadius)))) (+ (+ (Transformation|GetActorLocation) (* (+ (* (Transformation|GetActorForwardVector) (Math|Trig|Cos(Degrees) _returnvalue)) (* (Transformation|GetActorRightVector) (Math|Trig|Sin(Degrees) _returnvalue))) (* (Math|Float|Power (/ (Math|Conversions|ToFloat(Integer) (+ _index 1)) (Math|Conversions|ToFloat(Integer) _amount)) (Variables|Base|GetRatio)) (Variables|Base|GetRadius)))) (* (Transformation|GetActorUpVector) -65535.0)) (Variables|Base|GetTraceTypes) false 0 "None"))
          (if _returnvalue_3
            (bind _returnvalue_4 (AddComponent|AddChildActorComponent false (Class|KismetMathLibrary|ConvertTransformtoRelative (Transformation|GetActorTransform) (CallFunction|CombineTransform (Math|Transform|MakeTransform (CallFunction|RandomVectorSeeded (Variables|Random|GetMinRandomLocation) (Variables|Random|GetMaxRandomLocation) _seed_4) (CallFunction|RandomRotSeeded (Variables|Random|GetMinRandomRotation) (Variables|Random|GetMaxRandomRotation) _seed_4) (CallFunction|RandomVectorSeeded (Variables|Random|GetMinRandomScale) (Variables|Random|GetMaxRandomScale) _seed_4)) (Math|Transform|MakeTransform (+ (* (.ImpactNormal (Collision|BreakHitResult _outhit)) (Variables|Base|GetHeight)) (.ImpactPoint (Collision|BreakHitResult _outhit)) "") (Math|Rotator|SelectRotator (Math|Rotator|MakeRotfromZ (.ImpactNormal (Collision|BreakHitResult _outhit))) (Math|Rotator|SelectRotator (Transformation|GetActorRotation) (Variables|Base|GetBaseRotation) (Variables|Base|GetUseActorDir)) (Variables|Base|GetUseNormal)) (Variables|Base|GetBaseScale))))))
            (switch Utilities|FlowControl|Switch|SwitchonESelect (Variables|Base|GetMeshSelection)
              (:NewEnumerator0
                (ChildActorComponent|SetChildActorClass _returnvalue_4 (Utilities|Array|Get(acopy) (Variables|Base|GetClasses) (LocalVariables|GetpIndex)))
                (LocalVariables|SetpIndex (Math|Integer|%(Integer) (+ (LocalVariables|GetpIndex) 1) (Utilities|Array|Length (Variables|Base|GetClasses)))))
              (:NewEnumerator1
                (ChildActorComponent|SetChildActorClass _returnvalue_4 (Utilities|RandomItemSeeded (Variables|Base|GetClasses) (Variables|Base|GetSeed))))))
          (else
            (bind _returnvalue_5 (AddComponent|AddChildActorComponent false (CallFunction|CombineTransform (Math|Transform|MakeTransform (+ (* (Math|Vector|MakeVector (Math|Trig|Cos(Degrees) _returnvalue_2) (Math|Trig|Sin(Degrees) _returnvalue_2) 0.0) (* (Math|Float|Power (/ (Math|Conversions|ToFloat(Integer) (+ _index 1)) (Math|Conversions|ToFloat(Integer) _amount)) (Variables|Base|GetRatio)) (Variables|Base|GetRadius))) (Math|Vector|MakeVector 0.0 0.0 (Math|Random|RandomFloatinRangefromStream 0.0 (Variables|Base|GetHeight) (Variables|Base|GetSeed)))) (Variables|Base|GetBaseRotation) (Variables|Base|GetBaseScale)) (Math|Transform|MakeTransform (CallFunction|RandomVectorSeeded (Variables|Random|GetMinRandomLocation) (Variables|Random|GetMaxRandomLocation) _seed) (CallFunction|RandomRotSeeded (Variables|Random|GetMinRandomRotation) (Variables|Random|GetMaxRandomRotation) _seed) (CallFunction|RandomVectorSeeded (Variables|Random|GetMinRandomScale) (Variables|Random|GetMaxRandomScale) _seed)))))
            (switch Utilities|FlowControl|Switch|SwitchonESelect (Variables|Base|GetMeshSelection)
              (:NewEnumerator0
                (ChildActorComponent|SetChildActorClass _returnvalue_5 (Utilities|Array|Get(acopy) (Variables|Base|GetClasses) (LocalVariables|GetpIndex)))
                (LocalVariables|SetpIndex (Math|Integer|%(Integer) (+ (LocalVariables|GetpIndex) 1) (Utilities|Array|Length (Variables|Base|GetClasses)))))
              (:NewEnumerator1
                (ChildActorComponent|SetChildActorClass _returnvalue_5 (Utilities|RandomItemSeeded (Variables|Base|GetClasses) (Variables|Base|GetSeed)))))))))))